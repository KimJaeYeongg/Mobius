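; BP_Component is a helper Blueprint for cursor-driven aiming: mouse world location, player facing and a dash target decal.
; PlayerRotateMouse intersects the deprojected cursor ray with a horizontal plane at the character's height, traces to it, and sets control yaw toward the result.
; MouseDecal aligns the decal to the surface under the cursor, returning IsValidDash below a fixed height limit.
; BeginPlay and Tick are empty; decal hiding is unconnected.
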(event EventBeginPlay)

(event EventTick
  (params (DeltaSeconds :type Float%20%28single-precision%29)))

(fn GetMouseLocation
  (params (Controller :type Player%20Controller%20Object%20Reference))
  (return (.Location (Collision|BreakHitResult (.HitResult (Game|Player|GetHitResultUnderCursorbyChannel Controller "TraceTypeQuery2" true))))))

(fn PlayerRotateMouse
  (params (PlayerController :type Player%20Controller%20Object%20Reference) (PlayerCharacter :type Actor%20Object%20Reference))
  (bind (_worldlocation _worlddirection) (Game|Player|ConvertMouseLocationToWorldSpace PlayerController))
  (LocalVariables|SetPlayerController_Local PlayerController)
  (LocalVariables|SetPlayerCharater_Local PlayerCharacter)
  (bind _outhit (Collision|LineTraceByChannel _worldlocation (.Intersection (Class|KismetMathLibrary|LinePlaneIntersectionOriginNormal _worldlocation (|((MouseDir*TraceLenght)+MouseLoc) _worlddirection (LocalVariables|GetDistance%20Hit%20Mouse) _worldlocation) (Transformation|GetActorLocation (LocalVariables|GetPlayerCharater_Local)) "0, 0,1.000000")) "TraceTypeQuery2" false 0 "None"))
  (Variables|Default|SetMouseLocation (Math|Vector|SelectVector (.ImpactPoint (Collision|BreakHitResult _outhit)) (.TraceEnd (Collision|BreakHitResult _outhit)) (.bBlockingHit (Collision|BreakHitResult _outhit))))
  ;[1 1 1] Rotate Player axle Z
  (Pawn|SetControlRotation (LocalVariables|GetPlayerController_Local) (Math|Rotator|MakeRotator 0.0 0.0 (.yaw (Math|Rotator|FindLookatRotation (Transformation|GetActorLocation (LocalVariables|GetPlayerCharater_Local)) (Math|Vector|SelectVector (.ImpactPoint (Collision|BreakHitResult _outhit)) (.TraceEnd (Collision|BreakHitResult _outhit)) (.bBlockingHit (Collision|BreakHitResult _outhit))))))))

(fn MouseDecal
  (params (DecalMultDash :type Scene%20Component%20Object%20Reference) (PlayerController :type Player%20Controller%20Object%20Reference))
  (bind _hitresult (Game|Player|GetHitResultUnderCursorbyChannel PlayerController "TraceTypeQuery1" true))
  (bind (_bblockinghit _binitialoverlap _time _distance _location _impactpoint _normal _impactnormal) (Collision|BreakHitResult _hitresult))
  (Transformation|SetWorldLocationAndRotation DecalMultDash (Math|Vector|MakeVector (.x _location) (.y _location) (.z _location)) (Math|Rotator|MakeRotationfromAxes _impactnormal "0, 0, 0" "0, 0, 0") false false)
  (if (<= (.z _location) 91.0)
    (return (Variables|Default|GetIsValidDash?))))