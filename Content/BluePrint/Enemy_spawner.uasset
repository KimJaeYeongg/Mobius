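; Enemy spawner actor that spawns queued enemy classes at its own transform, passing the wave number to each enemy's max health setter.
; A looping timer pops the queue, while newly queued enemies trigger an immediate spawn attempt if no enemy overlaps its sphere.
; It binds to each spawn's destruction and has an event that reports defeats to the third-person GameMode.
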(event `self.ReceiveBeginPlay`
  (`KismetSystemLibrary.K2_SetTimerDelegate` (delegate `TryToSpawn`) 2.0 true))

(event `TryToSpawn`
  (`self.SpawnEnemy`))

(event `OnEnemyDefeated`
  (bind _asbp_third_person_game_mode (cast `/Game/ThirdPerson/Blueprints/BP_ThirdPersonGameMode` (`GameplayStatics.GetGameMode`)))
  (`/Game/ThirdPerson/Blueprints/BP_ThirdPersonGameMode.OnEnemyDefeated` _asbp_third_person_game_mode))

(fn `AddEnemyToQueue`
  (params (EnemyClass :type "/Game/BluePrint/Enemy Class Reference (by ref)"))
  (`KismetArrayLibrary.Array_Add` (`self.EnemyQueue`) EnemyClass)
  (if (not (`KismetArrayLibrary.Array_IsValidIndex` (`PrimitiveComponent.GetOverlappingActors` (`self.Sphere`) "/Game/BluePrint/Enemy.Enemy_C")))
    (`self.SpawnEnemy`)))

(fn `IncreaseHealth`)

(fn `SpawnEnemy`
  (returns (Success :type Boolean))
  (if (`KismetArrayLibrary.Array_IsValidIndex` (`self.EnemyQueue`))
    (bind _returnvalue (`|SpawnActorFromClass` (`|GetArrayItem` (`self.EnemyQueue`)) (`self.GetTransform`) "AdjustIfPossibleButAlwaysSpawn" "MultiplyWithRoot" null null))
    (`/Game/BluePrint/Enemy.Set Max Health` _returnvalue (`self.waveNum`))
    (add `/Game/BluePrint/Enemy.On Destroyed` _returnvalue (`|CreateDelegate` :!event `OnEnemyDefeated`))
    (`KismetArrayLibrary.Array_Remove` (`self.EnemyQueue`))
    (return true)
    (else
      (return false))))

(fn `UserConstructionScript`)