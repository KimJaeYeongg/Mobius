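; Boss enemy Blueprint that carries a weapon and periodically fires projectiles, with the player character passed as their target.
; On BeginPlay it sets its enemy type, attaches a spawned BP_Weapon to the right-hand socket and starts a looping Skill timer.
; Skill spawns a configurable projectile class at the AtkArrow transform and binds its impact event to Damage, which applies fixed damage to the actor hit.
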(event `self.ReceiveBeginPlay`
  (`parent.ReceiveBeginPlay`)
  (set `self.type` "Enemy3")
  (bind _returnvalue (`|SpawnActorFromClass` "/Game/joyeong/BP_Weapon.BP_Weapon_C" (`SceneComponent.GetSocketTransform` (`self.Mesh`) "RightHand소켓" "RTS_World") "Undefined" "MultiplyWithRoot" null null))
  (`self.K2_AttachToComponent` _returnvalue (`self.Mesh`) "RightHand소켓" "SnapToTarget" "SnapToTarget" "SnapToTarget" true)
  (`KismetSystemLibrary.K2_SetTimerDelegate` (delegate `Skill`) (`self.Frequency`) true))

(event `Skill`
  (bind _returnvalue (`GameplayStatics.GetActorOfClass` (`GameplayStatics.GetObjectClass` (`GameplayStatics.GetPlayerCharacter` 0))))
  (bind _returnvalue_2 (`|SpawnActorFromClass` (`self.projectileType`) (`SceneComponent.K2_GetComponentToWorld` (`self.AtkArrow`)) "Undefined" "MultiplyWithRoot" self 500.0 0.0 _returnvalue null))
  (add `/Game/BluePrint/Bp_projectile_Base.OnProjectileImpact` _returnvalue_2 (delegate `Damage`)))

(event `Damage`
  (params (`Other Actor` :type "Actor Object Reference") (Hit :type "HitResult Structure"))
  (`GameplayStatics.ApplyDamage` `Other Actor` 10.0))

(fn `UserConstructionScript`
  (`parent.UserConstructionScript`))