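; Enemy character that chases the player, attacks in melee and shows a widget health bar.
; SetMaxHealth scales health by wave and Type (BeginPlay sets Enemy1), then Operate starts a recursive AIMoveTo loop playing type-specific montages and applying damage.
; AnyDamage updates the bar and flashes the material; death triggers a random pickup drop at a ground trace and calls OnDestroyed.
; Hitting the player also deals delayed contact damage.
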(event `self.ReceiveBeginPlay`
  ;[1 1 1] 적 1로 설정
  (set `self.type` "Enemy1"))

(event `Operate`
  (bind _max_health (`self.Max Health`))
  ;[1 1 1] 몬스터 움직이기, 체력바 설정
  (`self.UpdateHealthBar`)
  (`self.move`)
  (bind _aswb_ai_health_bar (cast `/Game/BluePrint/WB_AiHealthBar` (`WidgetComponent.GetUserWidgetObject` (`self.HealthBar`))))
  (set `/Game/BluePrint/WB_AiHealthBar.MaxHealth` _max_health _aswb_ai_health_bar)
  (set `self.Health1` _max_health))

(event `move`
  ;[1 1 1] 코멘트
  (set `self.CanAttack` true)
  (`|AIMoveTo` self (0.0 0.0 0.0) (`GameplayStatics.GetPlayerCharacter` 0) 70.0
    (:`OnSuccess`
      (set `self.CanAttack` false)
      (if (`KismetStringLibrary.EqualEqual_StrStr` (`self.type`) "Enemy1")
        (bind _returnvalue (`self.PlayAnimMontage` "/Game/scorpion/base_animation/Scorpion_Attack_Montage.Scorpion_Attack_Montage"))
        (bind _asbp_third_person_character (cast `/Game/ThirdPerson/Blueprints/BP_ThirdPersonCharacter` (`GameplayStatics.GetPlayerCharacter` 0)))
        (`GameplayStatics.ApplyDamage` _asbp_third_person_character (`self.BaseDamage`) null self)
        (`KismetSystemLibrary.Delay` _returnvalue)
        (set `self.CanAttack` true)
        (`self.move`)
        (elif (`KismetStringLibrary.EqualEqual_StrStr` (`self.type`) "Enemy2")
          (bind _returnvalue_2 (`self.PlayAnimMontage` "/Game/scorpion/elite_animation/Scorpion2_Attack_Montage.Scorpion2_Attack_Montage"))
          (bind _asbp_third_person_character_2 (cast `/Game/ThirdPerson/Blueprints/BP_ThirdPersonCharacter` (`GameplayStatics.GetPlayerCharacter` 0)))
          (`GameplayStatics.ApplyDamage` _asbp_third_person_character_2 (`self.BaseDamage`) null self)
          (`KismetSystemLibrary.Delay` _returnvalue_2)
          (set `self.CanAttack` true)
          (`self.move`)
          (elif (`KismetStringLibrary.EqualEqual_StrStr` (`self.type`) "Enemy3")
            (bind _returnvalue_3 (`self.PlayAnimMontage` "/Game/Horus2/Animation/Horus_Attack_Montage.Horus_Attack_Montage"))
            (bind _asbp_third_person_character_3 (cast `/Game/ThirdPerson/Blueprints/BP_ThirdPersonCharacter` (`GameplayStatics.GetPlayerCharacter` 0)))
            (`GameplayStatics.ApplyDamage` _asbp_third_person_character_3 (`self.BaseDamage`) null self)
            (`KismetSystemLibrary.Delay` _returnvalue_3)
            (set `self.CanAttack` true)
            (`self.move`)))))
    (:`OnFail`
      (`KismetSystemLibrary.Delay` 0.1)
      (`self.move`))))

(event `self.ReceiveAnyDamage`
  (params (Damage :type "Float (single-precision)") (DamageType :type "DamageType Object Reference") (InstigatedBy :type "Controller Object Reference") (DamageCauser :type "Actor Object Reference"))
  ;[1 1 1] 공격 당했을 때 체력바 줄어듬, 체력 0 일때 사망
  (bind _output_get (set `self.Health1` (- (`self.Health1`) Damage)))
  (bind _aswb_ai_health_bar (cast `/Game/BluePrint/WB_AiHealthBar` (`WidgetComponent.GetUserWidgetObject` (`self.HealthBar`))))
  (`self.ChangeDamageColor`)
  (set `/Game/BluePrint/WB_AiHealthBar.Health` _output_get _aswb_ai_health_bar)
  (if (<= _output_get 0.0)
    (`self.Drop Loot`)
    (`self.K2_DestroyActor`)
    (`self.On Destroyed`)))

(event `ChangeDamageColor`
  ;[1 1 1] 피격시 색상 변경
  (`PrimitiveComponent.SetMaterial` (`self.Mesh`) 0 "/Game/StarterContent/Materials/M_AssetPlatform.M_AssetPlatform")
  (`KismetSystemLibrary.Delay` 0.05)
  (`PrimitiveComponent.SetMaterial` (`self.Mesh`) 0 null)
  (`KismetSystemLibrary.Delay` 0.05)
  (`PrimitiveComponent.SetMaterial` (`self.Mesh`) 0 "/Game/StarterContent/Materials/M_AssetPlatform.M_AssetPlatform")
  (`KismetSystemLibrary.Delay` 0.05)
  (`PrimitiveComponent.SetMaterial` (`self.Mesh`) 0 null))

(event `self.ReceiveHit`
  (params (MyComp :type "PrimitiveComponent Object Reference") (Other :type "Actor Object Reference") (OtherComp :type "PrimitiveComponent Object Reference") (bSelfMoved :type Boolean) (HitLocation :type "Vector Structure") (HitNormal :type "Vector Structure") (NormalImpulse :type "Vector Structure") (Hit :type "HitResult Structure (by ref)"))
  ;[1 1 1] 충돌 시 데미지 줌
  (cast `/Game/ThirdPerson/Blueprints/BP_ThirdPersonCharacter` Other)
  (if (`self.ActorHasTag` Other "Player")
    (`KismetSystemLibrary.Delay` 1.0)
    (`GameplayStatics.ApplyDamage` Other (`self.BaseDamage`) null self)))

(event `Drop Loot`
  (bind _returnvalue (`self.K2_GetActorLocation`))
  ;[1 1 1] 랜덤 아이템 생성
  (bind _outhit (`KismetSystemLibrary.LineTraceSingle` _returnvalue (- _returnvalue (0.0 0.0 100.0)) "TraceTypeQuery1" false (`|MakeArray` (`GameplayStatics.GetPlayerCharacter` 0) :!type "Actor Object Reference")))
  (if (<= (`KismetMathLibrary.RandomFloatInRange` 0.0 1.0) 0.1)
    (`|SpawnActorFromClass` (select `int` (`KismetMathLibrary.RandomInteger` 4) :`0` "/Game/BluePrint/HealthItemBP.HealthItemBP_C" :`1` "/Game/BluePrint/IncreaseAtkBP.IncreaseAtkBP_C" :`2` "/Game/BluePrint/PcSpeedBp.PcSpeedBp_C" :`3` "/Game/BluePrint/BarrierBP.BarrierBP_C" :!type "Actor Class Reference") (`KismetMathLibrary.MakeTransform` (`.Location` (`GameplayStatics.BreakHitResult` _outhit)) (`KismetMathLibrary.MakeRotator` 0.0 0.0 (`KismetMathLibrary.RandomFloatInRange` 0.0 360.0))) "AdjustIfPossibleButDontSpawnIfColliding" "MultiplyWithRoot" null null)))

(fn `CurrentHealthBar`
  (bind _aswb_ai_health_bar (cast `/Game/BluePrint/WB_AiHealthBar` (`WidgetComponent.GetUserWidgetObject` (`self.HealthBar`))))
  (set `/Game/BluePrint/WB_AiHealthBar.MaxHealth` (+ (`self.Max Health`) (`self.IncreaseHealth`)) _aswb_ai_health_bar)
  (return))

(fn `Set Max Health`
  (params (wave :type Integer))
  (if (`KismetStringLibrary.EqualEqual_StrStr` (`self.type`) "Enemy1")
    (bind _output_get (set `self.Max Health` (+ (`self.Max Health`) (* wave 5))))
    (set `self.Health1` _output_get)
    (`self.Operate` :!label _label)
    (elif (`KismetStringLibrary.EqualEqual_StrStr` (`self.type`) "Enemy2")
      (bind _output_get_2 (set `self.Max Health` (+ (`self.Max Health`) (* wave 10))))
      (set `self.Health1` _output_get_2)
      (goto _label)
      (elif (`KismetStringLibrary.EqualEqual_StrStr` (`self.type`) "Enemy3")
        (bind _output_get_3 (set `self.Max Health` (+ (`self.Max Health`) (* wave 200))))
        (set `self.Health1` _output_get_3)
        (goto _label)))))

(fn `UpdateHealthBar`
  (bind _aswb_ai_health_bar (cast `/Game/BluePrint/WB_AiHealthBar` (`WidgetComponent.GetUserWidgetObject` (`self.HealthBar`))))
  (set `/Game/BluePrint/WB_AiHealthBar.Health` (`self.Health1`) _aswb_ai_health_bar)
  (return))

(fn `UserConstructionScript`)