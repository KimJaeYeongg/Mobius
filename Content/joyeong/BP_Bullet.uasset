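; BP_Bullet is a projectile that scales its effect and damage with the game mode's wave number.
; On spawn it finds the third-person character, then Attack activates one of three bullet components by wave tier through wave 15.
; The higher two tiers also overwrite the character's BulletDamage.
; A sphere hit spawns an effect, destroys the bullet and applies that damage to the hit actor.
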(event `self.ReceiveBeginPlay`
  (bind _returnvalue (`GameplayStatics.GetActorOfClass` "/Game/ThirdPerson/Blueprints/BP_ThirdPersonCharacter.BP_ThirdPersonCharacter_C"))
  (`/Engine/EditorBlueprintResources/StandardMacros.IsValid` _returnvalue
    (:`Is Valid`
      (set `self.ThirdCharacter` _returnvalue)
      (`self.Attack`))))

(event `self.Sphere.OnComponentHit`
  (params (HitComponent :type "PrimitiveComponent Object Reference") (OtherActor :type "Actor Object Reference") (OtherComp :type "PrimitiveComponent Object Reference") (NormalImpulse :type "Vector Structure") (Hit :type "HitResult Structure (by ref)"))
  (`NiagaraFunctionLibrary.SpawnSystemAtLocation` (`self.HitEffect`) (`SceneComponent.K2_GetComponentLocation` (`self.Bullet1`)))
  (`PrimitiveComponent.AddImpulseAtLocation` OtherComp (0.0 0.0 0.0) (0.0 0.0 0.0) "None")
  (`self.K2_DestroyActor`)
  (`GameplayStatics.ApplyDamage` OtherActor (`/Game/ThirdPerson/Blueprints/BP_ThirdPersonCharacter.bulletDamage` (`self.ThirdCharacter`))))

(fn `Attack`
  (bind _asbp_third_person_game_mode (cast `/Game/ThirdPerson/Blueprints/BP_ThirdPersonGameMode` (`GameplayStatics.GetGameMode`)))
  (bind _wavenumber (`/Game/ThirdPerson/Blueprints/BP_ThirdPersonGameMode.WaveNumber` _asbp_third_person_game_mode))
  (if (<= _wavenumber 5)
    (`ActorComponent.Activate` (`self.Bullet1`) false)
    (elif (and (>= _wavenumber 6) (<= _wavenumber 10))
      (bind _asbp_third_person_character (cast `/Game/ThirdPerson/Blueprints/BP_ThirdPersonCharacter` (`GameplayStatics.GetPlayerCharacter` 0)))
      (set `/Game/ThirdPerson/Blueprints/BP_ThirdPersonCharacter.bulletDamage` 20.0 _asbp_third_person_character)
      (`ActorComponent.Activate` (`self.Bullet2`) false)
      (elif (and (>= _wavenumber 11) (<= _wavenumber 15))
        (bind _asbp_third_person_character_2 (cast `/Game/ThirdPerson/Blueprints/BP_ThirdPersonCharacter` (`GameplayStatics.GetPlayerCharacter` 0)))
        (set `/Game/ThirdPerson/Blueprints/BP_ThirdPersonCharacter.bulletDamage` 30.0 _asbp_third_person_character_2)
        (`ActorComponent.Activate` (`self.Bullet3`) false)))))

(fn `UserConstructionScript`)